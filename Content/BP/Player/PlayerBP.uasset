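; Player character Blueprint for a side-scrolling platformer, with movement along X, wall sliding, wall jumps and limited jetpack air jumps.
; A per-tick sphere trace detects walls, lowering gravity and clamping slide speed, while a short post-jump flag suspends that clamp.
; Timelines and smoothed fall speed combine with Health to squash, stretch and scale the cube mesh.
; Zero Health deactivates movement, and BeginPlay adds the player widget.
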(event EventBeginPlay
  (bind _returnvalue (UserInterface|CreateWidget "/Game/BP/Player/PlayerWidget.PlayerWidget_C" 0 self))
  (UserInterface|Viewport|AddtoViewport _returnvalue 0))

(event EventTick
  (params (DeltaSeconds :type Float%20%28single-precision%29))
  (bind _returnvalue (Transformation|GetActorLocation))
  (bind _returnvalue_2 (Transformation|GetActorLocation))
  (bind _cube (Variables|Default|GetCube))
  (bind _charactermovement (Variables|Character|GetCharacterMovement))
  (Utilities|FlowControl|Sequence
    (:then_0
      (Transformation|SetActorLocation (Math|Vector|MakeVector (.x _returnvalue_2) 0.0 (.z _returnvalue_2)) false false)
      (bind (_outhit _returnvalue_3) (Collision|SphereTraceByChannel _returnvalue _returnvalue 7e+01 "TraceTypeQuery2" false 0 "None"))
      (bind _output_get (Variables|Default|SetOnWall _returnvalue_3))
      (Variables|Default|SetWall%20Normal (.Normal (Collision|BreakHitResult _outhit)))
      (Variables|/Script/Engine.CharacterMovementComponent|SetGravityScale (Variables|Character|GetCharacterMovement) (Math|Float|SelectFloat 0.1 3.0 _output_get))
      (if (and (Variables|Default|GetOnWall) (not (Variables|Default|GetJustJumped)))
        (Variables|/Script/Engine.MovementComponent|SetVelocity _charactermovement (Math|Vector|MakeVector (.x (Variables|/Script/Engine.MovementComponent|GetVelocity _charactermovement)) (.x (Variables|/Script/Engine.MovementComponent|GetVelocity _charactermovement)) (Math|Float|Clamp(Float) (.z (Variables|/Script/Engine.MovementComponent|GetVelocity _charactermovement)) -2e+02 5e+01)))
        (if (AI|Components|NavMovement|IsMovingonGround (Variables|Character|GetCharacterMovement))
          _)))
    (:then_1
      (if (Variables|Default|GetOnWall)
        (bind _newtrack_0 (Timeline|Timeline_0 Play)
          (:Update
            (Variables|Default|Setwallscale (Math|Vector|Lerp(Vector) "1.000000,1.000000,1.000000" "0.750000,0.750000,1.250000" _newtrack_0))))
        (else
          (Timeline|Timeline_0 Reverse))))
    (:then_2
      (Transformation|SetRelativeScale3D _cube (* (Variables|Default|Getwallscale) (Variables|Default|Getjumpscale) (Math|Vector|Lerp(Vector) "1.000000,1.000000,1.000000" "0.750000,0.750000,1.500000" (Math|Float|Clamp(Float) (/ (Variables|Default|Getfallscale) -2.2e+03))) (Math|Conversions|ToVector(Float) (Variables|Default|GetHealth))))
      (Variables|Default|Setfallscale (Math|Float|Lerp (Variables|Default|Getfallscale) (.z (Variables|/Script/Engine.MovementComponent|GetVelocity (Variables|Character|GetCharacterMovement))) (* 15 (Utilities|Time|GetWorldDeltaSeconds))))
      (Transformation|SetRelativeRotation _cube (Math|Rotator|MakeRotator 0.0 0.0 (Math|Float|Clamp(Float) (/ (.x (Variables|/Script/Engine.MovementComponent|GetVelocity (Variables|Character|GetCharacterMovement))) -5.0) -9e+01 9e+01)) false false))
    (:then_3
      (if (<= (Variables|Default|GetHealth) 0.0)
        (Components|Activation|Deactivate (Variables|Character|GetCharacterMovement))))
    (:then_4
      (Rendering|SetVisibility (Variables|Default|GetStaticMesh) (> (Variables|Default|GetJetpackJumps) 0) false))))

(event Input|ActionEvents|InputActionJump
  (params (Key :type Key%20Structure :default "None"))
  (bind _returnvalue (Game|GetPlayerCameraManager 0))
  (bind _wall_normal (Variables|Default|GetWall%20Normal))
  (bind _returnvalue_2 (* _wall_normal 1200))
  (bind (_x _y) (Math|Vector|BreakVector _returnvalue_2))
  (:Pressed
    (if (> (Variables|Default|GetHealth) 0.0)
      (if (AI|Components|NavMovement|IsMovingonGround (Variables|Character|GetCharacterMovement))
        (Character|LaunchCharacter "0, 0,1750.000000" false true :!label _label)
        (CameraShakes|StartCameraShake _returnvalue "/Game/BP/Player/CameraShake/Jump.Jump_C" 1.0 "CameraLocal" "0, 0, 0")
        (bind _newtrack_0 (Timeline|Timeline_1 PlayFromStart)
          (:Update
            (Variables|Default|Setjumpscale (Math|Vector|Lerp(Vector) "1.000000,1.000000,1.000000" "1.500000,1.500000,0.500000" _newtrack_0))))
        (elif (Variables|Default|GetOnWall)
          (Utilities|FlowControl|Sequence
            (:then_0
              (Character|LaunchCharacter (Math|Vector|MakeVector _x _y 1.75e+03) false true)
              (CameraShakes|StartCameraShake _returnvalue "/Game/BP/Player/CameraShake/Jump.Jump_C" 1.0 "CameraLocal" "0, 0, 0")
              (Variables|Default|SetJustJumped true)
              (Utilities|FlowControl|Delay 0.2)
              (Variables|Default|SetJustJumped false))
            (:then_1
              (Timeline|Timeline_1 PlayFromStart)))
          (elif (> (Variables|Default|GetJetpackJumps) 0)
            (Math|Integer|DecrementInt (Variables|Default|GetJetpackJumps)
              (:%20%20
                (Components|Activation|Activate (Variables|Default|GetJetpackDust) true)
                (goto _label)))))))))

(event Input|AxisEvents|InputAxisRight
  (params (AxisValue :type Float%20%28single-precision%29))
  (Pawn|Input|AddMovementInput (Math|Vector|MakeVector 1.0 0.0 0.0) AxisValue false))

(fn ConstructionScript)